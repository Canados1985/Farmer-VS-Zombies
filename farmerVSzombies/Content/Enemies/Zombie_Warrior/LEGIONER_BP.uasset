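; Legioner zombie warrior enemy that hunts the player, attacks at close range or at fences, and takes bullet damage.
; BeginPlay attaches one random weapon, shield and helmet loadout and starts a wander timer, whose function name differs from the wander event's.
; Pawn sensing drives AIMoveTo, while overlaps and Tick set state flags for attacks and hit stuns.
; Death awards a kill, may drop a coin or rare star, then sinks and destroys the body.
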(event OnHearNoise(PawnSensing_Own)
  (params (Instigator :type Pawn%20Object%20Reference) (Location :type Vector%20%28by%20ref%29 :default "0, 0, 0") (Volume :type Float%20%28single-precision%29))
  (bind _asthird_person_character (Utilities|Casting|CastToThirdPersonCharacter Instigator))
  (AI|AIMoveTo self (Transformation|GetWorldLocation (Variables|/Script/Engine.Character|GetCapsuleComponent _asthird_person_character)) 0 5.0 false))

(event OnSeePawn(PawnSensing_Own)
  (params (Pawn :type Pawn%20Object%20Reference))
  ;[1 1 1] SEEING ACTORS
  (if (Math|Boolean|ANDBoolean (not (Variables|Default|GetLegioner_Attacking)) (not (Variables|Default|GetLegioner_Gets_Shot)) (not (Variables|Default|GetLegioner_Dead_With_Shield)) (not (Variables|Default|GetLegioner_Is_Kicking)))
    (Utilities|FlowControl|Sequence
      (:then_0
        (bind _asthird_person_character (Utilities|Casting|CastToThirdPersonCharacter Pawn))
        (if (Math|Boolean|ANDBoolean (not (Variables|Default|GetLegioner_Dead_With_Shield)) (not (Variables|/Game/ThirdPersonBP/Character_BP/ThirdPersonCharacter.ThirdPersonCharacter_C|GetCharacter_Is_Dead _asthird_person_character)) (not (Variables|Default|GetLegioner_Is_Kicking)))
          (AI|AIMoveTo self (Transformation|GetWorldLocation (Variables|/Script/Engine.Character|GetCapsuleComponent _asthird_person_character)) 0 5.0 false)))
      (:then_1
        (bind _asbp_fence (Utilities|Casting|CastToBP_FENCE Pawn))
        (if (Math|Boolean|ANDBoolean (not (Variables|Default|GetLegioner_Attacking)) (not (Variables|Default|GetLegioner_Gets_Shot)) (not (Variables|Default|GetLegioner_Dead_With_Shield)) (not (Variables|/Game/ThirdPersonBP/Env/Fence/BP_FENCE.BP_FENCE_C|GetFense_Is_destroyed _asbp_fence)))
          (AI|AIMoveTo self (Transformation|GetWorldLocation (Variables|/Game/ThirdPersonBP/Env/Fence/BP_FENCE.BP_FENCE_C|GetCapsule _asbp_fence)) 0 5.0 false)
          (else
            (Variables|Default|SetLegioner_Speed 1.5e+02)
            (Variables|/Script/Engine.CharacterMovementComponent|SetMaxWalkSpeed (Variables|Character|GetCharacterMovement) 1.5e+02)))))))

(event Custom|Legioner_Gets_Bullet_Event
  (bind _mesh (Variables|Character|GetMesh))
  (bind _returnvalue (Transformation|GetWorldLocation _mesh))
  (bind (_x _y _z) (Math|Vector|BreakVector _returnvalue))
  ;[1 1 1] LEGIONER GETS SHOT
  (Variables|Default|SetLegioner_Gets_Shot true)
  (Variables|Default|SetLegioner_Is_Kicking false)
  (Variables|Default|SetLegioner_Attacking false)
  (bind _returnvalue_2 (Effects|SpawnEmitterAttached "/Game/StarterContent/Particles/NewestBlood.NewestBlood" (Variables|Default|GetBlood) "LEGIONER" (Math|Vector|MakeVector _x _y (+ _z 5e+01)) "0, 0, 0" "5.000000,5.000000,5.000000" "KeepWorldPosition" false))
  (Variables|/Script/AIModule.PawnSensingComponent|SetSightRadius (Variables|Default|GetPawnSensing_Own) 0.0)
  (Variables|Default|SetLegioner_Speed 0.0)
  (Variables|/Script/Engine.CharacterMovementComponent|SetMaxWalkSpeed (Variables|Character|GetCharacterMovement) 0.0)
  (Rendering|SetVisibility _returnvalue_2 false false)
  (Audio|PlaySoundatLocation "/Game/Enemies/Zombie/Sounds/bullet_impact_body_Cue.bullet_impact_body_Cue" (Transformation|GetWorldLocation (Variables|Default|GetCapsuleComponent)))
  (Variables|Default|SetLegioner_Life (- (Variables|Default|GetLegioner_Life) 35))
  (bind _aszombie_widjet (Utilities|Casting|CastToZombie_WIDJET (UserInterface|GetUserWidgetObject (Variables|Default|GetWidget))))
  (Variables|/Game/Enemies/Zombie/Zombie_WIDJET.Zombie_WIDJET_C|SetZombie_Life_Widjet _aszombie_widjet (- (Variables|/Game/Enemies/Zombie/Zombie_WIDJET.Zombie_WIDJET_C|GetZombie_Life_Widjet _aszombie_widjet) 35))
  (Utilities|FlowControl|Delay 0.5)
  (Variables|Default|SetLegioner_Gets_Shot false)
  (Utilities|FlowControl|Delay 0.5)
  (Variables|Default|SetLegioner_Speed 1.5e+02)
  (Variables|/Script/Engine.CharacterMovementComponent|SetMaxWalkSpeed (Variables|Character|GetCharacterMovement) 1.5e+02)
  (Variables|/Script/AIModule.PawnSensingComponent|SetSightRadius (Variables|Default|GetPawnSensing_Own) 1.5e+03))

(event Custom|Attack%20Character
  (Variables|Default|SetLegioner_Speed 0.0)
  (Variables|/Script/Engine.CharacterMovementComponent|SetMaxWalkSpeed (Variables|Character|GetCharacterMovement) 0.0)
  (Variables|Default|SetSingle_Sword_Attack true)
  (Utilities|FlowControl|Delay 1.0)
  (Audio|SpawnSoundatLocation "/Game/Enemies/Zombie_Warrior/Sound/sword_Cue.sword_Cue" (Transformation|GetWorldLocation (Variables|Character|GetMesh)))
  (Utilities|FlowControl|Delay 2.0)
  (Variables|Default|SetSingle_Sword_Attack false))

(event Custom|Legioner_New_Position_Event
  (bind _capsulecomponent (Variables|Default|GetCapsuleComponent))
  (bind _returnvalue (Transformation|GetWorldLocation _capsulecomponent))
  (bind (_x _y _z) (Math|Vector|BreakVector _returnvalue))
  ;[1 1 1] BEGIN
  ;;[1 1 1] MOVING TO NEW POSITION
  (if (Math|Boolean|ANDBoolean (not (Variables|Default|GetLegioner_Attacking)) (not (Variables|Default|GetLegioner_Gets_Shot)) (not (Variables|Default|GetLegioner_Dead_With_Shield)) (not (Variables|Default|GetLegioner_Is_Kicking)) (not (Variables|Default|GetLegioner_Dead_Without_Shield)))
    (AI|AIMoveTo self (Math|Vector|MakeVector (+ (Math|Random|RandomFloatinRange -3e+03 2.5e+03) _x) (+ (Math|Random|RandomFloatinRange -2.3e+03 3.3e+03) _y) _z) 0 5.0 false)))

(event EventBeginPlay
  ;[1 1 1] BEGIN
  (Math|Integer|CompareInt (Math|Random|RandomIntegerinRange 0 10) 5
    (:>
      (Math|Integer|CompareInt (Math|Random|RandomIntegerinRange 0 10) 5
        (:>
          (Transformation|AttachComponentToComponent (Variables|Default|GetHelmet1) (Variables|Character|GetMesh) "HELMET" "SnapToTarget" "SnapToTarget" "SnapToTarget" true :!label _label)
          (Collision|SetActorEnableCollision true)
          (Transformation|AttachComponentToComponent (Variables|Default|GetSword) (Variables|Character|GetMesh) "GLADIUS_RIGHT_HAND" "SnapToTarget" "SnapToTarget" "SnapToTarget" true)
          (Collision|SetActorEnableCollision true)
          (Transformation|AttachComponentToComponent (Variables|Default|GetShield2) (Variables|Character|GetMesh) "SHIELD2_LEFT_HAND" "SnapToTarget" "SnapToTarget" "SnapToTarget" true)
          (Collision|SetActorEnableCollision true)
          (Utilities|FlowControl|Delay 0.2)
          (Components|DestroyComponent (Variables|Default|GetBarb_Helmet))
          (Collision|SetCollisionEnabled (Variables|Default|GetCapsuleComponent) "QueryAndPhysics"))
        (:==
          (goto _label))
        (:<
          (Transformation|AttachComponentToComponent (Variables|Default|GetBarb_Helmet) (Variables|Character|GetMesh) "HELMET3" "SnapToTarget" "SnapToTarget" "SnapToTarget" true)
          (Collision|SetActorEnableCollision true)
          (Transformation|AttachComponentToComponent (Variables|Default|GetBarb_axe) (Variables|Character|GetMesh) "BARB_AXE_RIGHT_HAND" "SnapToTarget" "SnapToTarget" "SnapToTarget" true)
          (Collision|SetActorEnableCollision true)
          (Transformation|AttachComponentToComponent (Variables|Default|GetBarb_Shied) (Variables|Character|GetMesh) "SHIELD_BARB_LEFT HAND" "SnapToTarget" "SnapToTarget" "SnapToTarget" true)
          (Collision|SetActorEnableCollision true)
          (Utilities|FlowControl|Delay 0.2)
          (Components|DestroyComponent (Variables|Default|GetHelmet2))
          (Collision|SetCollisionEnabled (Variables|Default|GetCapsuleComponent) "QueryAndPhysics"))))
    (:==
      (Transformation|AttachComponentToComponent (Variables|Default|GetHelmet1) (Variables|Character|GetMesh) "HELMET" "SnapToTarget" "SnapToTarget" "SnapToTarget" true)
      (Collision|SetActorEnableCollision true)
      (Transformation|AttachComponentToComponent (Variables|Default|GetSpear) (Variables|Character|GetMesh) "PIKE_RIGHT_HAND" "SnapToTarget" "SnapToTarget" "SnapToTarget" true)
      (Collision|SetActorEnableCollision true)
      (Transformation|AttachComponentToComponent (Variables|Default|GetMacShield) (Variables|Character|GetMesh) "SHIELD3_LEFT_HAND" "SnapToTarget" "SnapToTarget" "SnapToTarget" true)
      (Collision|SetActorEnableCollision true)
      (Utilities|FlowControl|Delay 0.2)
      (Components|DestroyComponent (Variables|Default|GetBarb_Helmet))
      (Collision|SetCollisionEnabled (Variables|Default|GetCapsuleComponent) "QueryAndPhysics"))
    (:<
      (Transformation|AttachComponentToComponent (Variables|Default|GetHelmet2) (Variables|Character|GetMesh) "HELMET2" "SnapToTarget" "SnapToTarget" "SnapToTarget" true)
      (Collision|SetActorEnableCollision true)
      (Transformation|AttachComponentToComponent (Variables|Default|GetSword) (Variables|Character|GetMesh) "GLADIUS_RIGHT_HAND" "SnapToTarget" "SnapToTarget" "SnapToTarget" true)
      (Collision|SetActorEnableCollision true)
      (Transformation|AttachComponentToComponent (Variables|Default|GetShield) (Variables|Character|GetMesh) "SHIELD_LEFT_HAND" "SnapToTarget" "SnapToTarget" "SnapToTarget" true)
      (Collision|SetActorEnableCollision true)
      (Utilities|FlowControl|Delay 0.2)
      (Components|DestroyComponent (Variables|Default|GetBarb_Helmet))
      (Collision|SetCollisionEnabled (Variables|Default|GetCapsuleComponent) "QueryAndPhysics")))
  (Utilities|Time|SetTimerbyFunctionName 0 "New_Position_Event" 3.0 true)
  (Components|Activation|SetActive (Variables|Default|GetBlood) false false))

(event Collision|EventActorBeginOverlap
  (params (OtherActor :type Actor%20Object%20Reference))
  ;[1 1 1] OVERLAPING WITH ACTORS
  (if (Actor|ActorHasTag OtherActor "BULLET")
    (Utilities|FlowControl|Delay 0.2)
    (CallFunction|LegionerGetsBulletEvent)
    (elif (Actor|ActorHasTag OtherActor "FENCE")
      (Variables|Default|SetLegioner_Speed 0.0)
      (Variables|/Script/Engine.CharacterMovementComponent|SetMaxWalkSpeed (Variables|Character|GetCharacterMovement) 0.0)
      (bind _asbp_fence (Utilities|Casting|CastToBP_FENCE OtherActor))
      (if (Math|Boolean|ANDBoolean (not (Variables|Default|GetLegioner_Dead_With_Shield)) (not (Variables|Default|GetLegioner_Dead_Without_Shield)) (not (Variables|/Game/ThirdPersonBP/Env/Fence/BP_FENCE.BP_FENCE_C|GetFense_Is_destroyed _asbp_fence)))
        (Variables|Default|SetLegioner_Near_Fence true)
        (Variables|Default|SetLegioner_Speed 0.0)
        (Variables|/Script/Engine.CharacterMovementComponent|SetMaxWalkSpeed (Variables|Character|GetCharacterMovement) 0.0)))))

(event Collision|EventActorEndOverlap
  (params (OtherActor :type Actor%20Object%20Reference))
  ;[1 1 1] END OVERLAP
  (if (Actor|ActorHasTag OtherActor "FENCE")
    (Variables|Default|SetLegioner_Speed 1.5e+02)
    (Variables|/Script/Engine.CharacterMovementComponent|SetMaxWalkSpeed (Variables|Character|GetCharacterMovement) 1.5e+02)
    (Variables|Default|SetLegioner_Is_Kicking false)
    (Variables|Default|SetLegioner_Near_Fence false)
    (elif (Actor|ActorHasTag OtherActor "BULLET")
      (Variables|Default|SetLegioner_Speed 1.5e+02)
      (Variables|/Script/Engine.CharacterMovementComponent|SetMaxWalkSpeed (Variables|Character|GetCharacterMovement) 1.5e+02)
      (Variables|Default|SetLegioner_Gets_Shot false))))

(event EventTick
  (params (DeltaSeconds :type Float%20%28single-precision%29))
  (bind _capsulecomponent (Variables|Default|GetCapsuleComponent))
  (bind _capsulecomponent_2 (Variables|Default|GetCapsuleComponent))
  (bind _mesh (Variables|Character|GetMesh))
  (bind _mesh_2 (Variables|Character|GetMesh))
  (bind _mesh_3 (Variables|Character|GetMesh))
  (bind _mesh_4 (Variables|Character|GetMesh))
  (bind _mesh_5 (Variables|Character|GetMesh))
  (bind _mesh_6 (Variables|Character|GetMesh))
  (bind _mesh_7 (Variables|Character|GetMesh))
  (bind _mesh_8 (Variables|Character|GetMesh))
  (bind _returnvalue (Transformation|GetWorldLocation _capsulecomponent))
  (bind _returnvalue_2 (Transformation|GetWorldLocation _capsulecomponent_2))
  (bind _returnvalue_3 (Transformation|GetWorldLocation _mesh))
  (bind _returnvalue_4 (Transformation|GetWorldLocation _mesh_2))
  (bind _returnvalue_5 (Transformation|GetWorldLocation _mesh_3))
  (bind _returnvalue_6 (Transformation|GetWorldLocation _mesh_4))
  (bind _returnvalue_7 (Transformation|GetWorldLocation _mesh_5))
  (bind _returnvalue_8 (Transformation|GetWorldLocation _mesh_6))
  (bind _returnvalue_9 (Transformation|GetWorldLocation _mesh_7))
  (bind _returnvalue_10 (Transformation|GetWorldLocation _mesh_8))
  (bind (_x _y _z) (Math|Vector|BreakVector _returnvalue))
  (bind (_x_2 _y_2 _z_2) (Math|Vector|BreakVector _returnvalue_2))
  (bind (_x_3 _y_3 _z_3) (Math|Vector|BreakVector _returnvalue_3))
  (bind (_x_4 _y_4 _z_4) (Math|Vector|BreakVector _returnvalue_4))
  (bind (_x_5 _y_5 _z_5) (Math|Vector|BreakVector _returnvalue_5))
  (bind (_x_6 _y_6 _z_6) (Math|Vector|BreakVector _returnvalue_6))
  (bind (_x_7 _y_7 _z_7) (Math|Vector|BreakVector _returnvalue_7))
  (bind (_x_8 _y_8 _z_8) (Math|Vector|BreakVector _returnvalue_8))
  (bind (_x_9 _y_9 _z_9) (Math|Vector|BreakVector _returnvalue_9))
  (bind (_x_10 _y_10 _z_10) (Math|Vector|BreakVector _returnvalue_10))
  (Math|Integer|CompareInt (Variables|Default|GetLegioner_Life)
    (:>
      (Math|Float|CompareFloat (Transformation|GetDistanceTo (Game|GetPlayerCharacter 0)) 2e+02
        (:>
          _)
        (:==
          (CallFunction|AttackCharacter :!label _label)
          (Utilities|FlowControl|Delay 4.0))
        (:<
          (goto _label)))
      (if (Math|Boolean|ANDBoolean (not (Variables|Default|GetLegioner_Attacking)) (not (Variables|Default|GetLegioner_Dead_With_Shield)) (not (Variables|Default|GetLegioner_Dead_Without_Shield)) (Variables|Default|GetLegioner_Near_Fence) (not (Variables|Default|GetLegioner_Gets_Shot)))
        (Variables|Default|SetSingle_Sword_Attack true)
        (Variables|Default|SetLegioner_Speed 0.0)
        (Variables|/Script/Engine.CharacterMovementComponent|SetMaxWalkSpeed (Variables|Character|GetCharacterMovement) 0.0)
        (Utilities|FlowControl|Delay 1.5)
        (Variables|Default|SetSingle_Sword_Attack false)
        (bind _asbp_fence (Utilities|Casting|CastToBP_FENCE (stale Collision|EventActorBeginOverlap OtherActor)))
        (if (Variables|/Game/ThirdPersonBP/Env/Fence/BP_FENCE.BP_FENCE_C|GetFense_Is_destroyed _asbp_fence)
          (Utilities|FlowControl|Delay 1.0)
          (Variables|Default|SetSingle_Sword_Attack false :!label _label_2)
          (Utilities|FlowControl|Delay 1.5)
          (Variables|Default|SetLegioner_Speed 1.5e+02)
          (Variables|/Script/Engine.CharacterMovementComponent|SetMaxWalkSpeed (Variables|Character|GetCharacterMovement) 1.5e+02)
          (bind _asbp_fence_2 (Utilities|Casting|CastToBP_FENCE (Components|GetOwner)))
          (if (Variables|/Game/ThirdPersonBP/Env/Fence/BP_FENCE.BP_FENCE_C|GetFense_Is_destroyed _asbp_fence_2)
            (Variables|Default|SetLegioner_Is_Kicking false)
            (Variables|/Script/AIModule.PawnSensingComponent|SetSightRadius (Variables|Default|GetPawnSensing_Own) 0.0)
            (Variables|Default|SetLegioner_Speed 1.5e+02)
            (Variables|/Script/Engine.CharacterMovementComponent|SetMaxWalkSpeed (Variables|Character|GetCharacterMovement) 1.5e+02)
            (Utilities|FlowControl|Delay 0.5)
            (Variables|/Script/AIModule.PawnSensingComponent|SetSightRadius (Variables|Default|GetPawnSensing_Own) 1.5e+03)))
        (else
          (Variables|Default|SetSingle_Sword_Attack false)
          (goto _label_2))))
    (:==
      (Math|Integer|CompareInt (Math|Random|RandomIntegerinRange 0 10) 5 :!label _label_3
        (:>
          (Variables|Default|SetLegioner_Dead_Without_Shield true :!label _label_4))
        (:==
          (goto _label_4))
        (:<
          (Variables|Default|SetLegioner_Dead_With_Shield true)))
      ;[1 1 1] LEGIONER IS DEAD WITH SHIELD
      (Class|Pawn|DetachfromControllerPendingDestroy)
      (Variables|Default|SetSingle_Sword_Attack false)
      (Variables|Default|SetLegioner_Gets_Shot false)
      (Variables|Default|SetLegioner_Attacking false)
      (Variables|Default|SetLegioner_Is_Kicking false)
      (Variables|Default|SetLegioner_Near_Fence false)
      (Variables|Default|SetShield_Durability_Counter 0)
      (Utilities|FlowControl|Sequence
        (:then_0
          (Utilities|FlowControl|DoOnce false
            (:Completed
              (bind _asthird_person_character (Utilities|Casting|CastToThirdPersonCharacter (Game|GetPlayerCharacter 0)))
              (Default|AddKillScore _asthird_person_character))))
        (:then_1
          (Rendering|SetVisibility (Variables|Default|GetWidget) false false)
          (Collision|SetCollisionEnabled (Variables|Default|GetCapsuleComponent) "NoCollision")
          (Components|Activation|SetActive (Variables|Default|GetPawnSensing_Own) false false)
          (Variables|Default|SetLegioner_Speed 0.0)
          (Variables|/Script/Engine.CharacterMovementComponent|SetMaxWalkSpeed (Variables|Character|GetCharacterMovement) 0.0)
          (Utilities|FlowControl|Delay 3.0)
          (Math|Integer|CompareInt (Math|Random|RandomIntegerinRange 0 100) 35
            (:>
              _)
            (:==
              (bind _returnvalue_11 (Game|SpawnActorfromClass "/Game/ThirdPersonBP/Env/Star/STAR_BP.STAR_BP_C" (Transformation|GetActorTransform) "Undefined" 0 0))
              (Transformation|SetWorldLocation (Variables|/Game/ThirdPersonBP/Env/Star/STAR_BP.STAR_BP_C|GetDefaultSceneRoot _returnvalue_11) (Math|Vector|MakeVector _x_2 _y_2 (- _z_2 1e+02)) false false))
            (:<
              (bind _returnvalue_12 (Game|SpawnActorfromClass "/Game/ThirdPersonBP/Env/Coin/COIN_BP.COIN_BP_C" (Transformation|GetActorTransform) "Undefined" 0 0))
              (Transformation|SetWorldLocation (Variables|/Game/ThirdPersonBP/Env/Coin/COIN_BP.COIN_BP_C|GetDefaultSceneRoot _returnvalue_12) (Math|Vector|MakeVector _x _y (- _z 1e+02)) false false)))
          (Transformation|SetWorldLocation (Variables|Character|GetMesh) (Math|Vector|MakeVector _x_3 _y_3 (- _z_3 5.0)) false false)
          (Utilities|FlowControl|Delay 0.3)
          (Transformation|SetWorldLocation (Variables|Character|GetMesh) (Math|Vector|MakeVector _x_4 _y_4 (- _z_4 5.0)) false false)
          (Utilities|FlowControl|Delay 0.3)
          (Transformation|SetWorldLocation (Variables|Character|GetMesh) (Math|Vector|MakeVector _x_5 _y_5 (- _z_5 5.0)) false false)
          (Utilities|FlowControl|Delay 0.3)
          (Transformation|SetWorldLocation (Variables|Character|GetMesh) (Math|Vector|MakeVector _x_6 _y_6 (- _z_6 5.0)) false false)
          (Utilities|FlowControl|Delay 0.3)
          (Transformation|SetWorldLocation (Variables|Character|GetMesh) (Math|Vector|MakeVector _x_7 _y_7 (- _z_7 5.0)) false false)
          (Utilities|FlowControl|Delay 0.3)
          (Transformation|SetWorldLocation (Variables|Character|GetMesh) (Math|Vector|MakeVector _x_8 _y_8 (- _z_8 5.0)) false false)
          (Utilities|FlowControl|Delay 0.3)
          (Transformation|SetWorldLocation (Variables|Character|GetMesh) (Math|Vector|MakeVector _x_9 _y_9 (- _z_9 5.0)) false false)
          (Utilities|FlowControl|Delay 0.3)
          (Transformation|SetWorldLocation (Variables|Character|GetMesh) (Math|Vector|MakeVector _x_10 _y_10 (- _z_10 5.0)) false false)
          (Utilities|FlowControl|Delay 0.3)
          (Actor|DestroyActor))))
    (:<
      (goto _label_3))))

(fn ConstructionScript
  (|CallParentFunction))